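; BP_GreenManRagdoll is an actor whose skeletal mesh is shown only outside the butterfly world.
; On BeginPlay it casts the game mode to GM_Butterfly, binds to its world-switch event and sets initial visibility from the IsButterfly flag.
; Each world switch then hides the mesh in the butterfly world and shows it otherwise, without propagating to child components.
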(event Custom|OnWorldSwitch_Event
  (params (ButterflyWorld :type Boolean))
  (Rendering|SetVisibility (Variables|Default|GetSkeletalMesh) (not ButterflyWorld) false))

(event EventBeginPlay
  (bind _asgm_butterfly (Utilities|Casting|CastToGM_Butterfly (Game|GetGameMode)))
  (EventDispatchers|AssignOnWorldSwitch _asgm_butterfly (delegate Custom|OnWorldSwitch_Event))
  (Rendering|SetVisibility (Variables|Default|GetSkeletalMesh) (not (Variables|/Game/ThirdPerson/Blueprints/GM_Butterfly.GM_Butterfly_C|GetIsButterfly _asgm_butterfly)) false))

(event Collision|EventActorBeginOverlap
  (params (OtherActor :type Actor%20Object%20Reference)))

(event EventTick
  (params (DeltaSeconds :type Float%20%28single-precision%29)))

(fn ConstructionScript)