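; Blood decal actor that shows only outside the butterfly world.
; On BeginPlay it casts the game mode to GM_Butterfly, binds to its OnWorldSwitch event and sets initial decal visibility from IsButterfly.
; Each world switch then hides the decal in the butterfly world and shows it otherwise.
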(event Custom|OnWorldSwitch_Event
  (params (ButterflyWorld :type Boolean))
  (Rendering|SetVisibility (Variables|Decal|GetDecal) (not ButterflyWorld) false))

(event EventBeginPlay
  (bind _asgm_butterfly (Utilities|Casting|CastToGM_Butterfly (Game|GetGameMode)))
  (EventDispatchers|AssignOnWorldSwitch _asgm_butterfly (delegate Custom|OnWorldSwitch_Event))
  (Rendering|SetVisibility (Variables|Decal|GetDecal) (not (Variables|/Game/ThirdPerson/Blueprints/GM_Butterfly.GM_Butterfly_C|GetIsButterfly _asgm_butterfly)) false))

(event EventTick
  (params (DeltaSeconds :type Float%20%28single-precision%29)))

(fn ConstructionScript)